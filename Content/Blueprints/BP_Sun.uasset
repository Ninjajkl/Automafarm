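; BP_Sun is an actor that rotates to match the farm game's time of day.
; On BeginPlay it reads the starting hour and time multiplier from FarmGameStateBase and binds to its hour-passed event.
; Tick advances a local second counter by scaled delta time and maps it to a full 360-degree pitch rotation per day.
; Each hour-passed event resyncs the counter to game time.
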(event Custom|HourPassed
  (params (GameTimePassed :type Timespan%20Structure))
  ;[0.07819 0.07819 0.07819] Align Sun Time With Game Time
  (Variables|TimePassed|SetCurrentSecond (Math|Float|%(Float) (Math|Timespan|GetTotalSeconds GameTimePassed) (Variables|TimeConstants|GetSecondsInDay))))

(event EventBeginPlay
  (bind _asfarm_game_state_base (Utilities|Casting|CastToFarmGameStateBase (Game|GetGameState)))
  (EventDispatchers|BindEventtoOnHourPassed _asfarm_game_state_base (delegate Custom|HourPassed))
  (Variables|TimePassed|SetTimeMultiplier (Variables|/Script/Automafarm.FarmGameStateBase|GetTimeMultiplier _asfarm_game_state_base))
  (Variables|TimePassed|SetCurrentSecond (* (Variables|/Script/Automafarm.FarmGameStateBase|GetStartingHour _asfarm_game_state_base) (Variables|TimeConstants|GetSecondsInHour))))

(event EventTick
  (params (DeltaSeconds :type Float%20%28single-precision%29))
  ;[0.07819 0.07819 0.07819] Rotate Sun
  (bind _output_get (Variables|TimePassed|SetCurrentSecond (Math|Float|%(Float) (+ (* DeltaSeconds (Variables|TimePassed|GetTimeMultiplier)) (Variables|TimePassed|GetCurrentSecond)) (Variables|TimeConstants|GetSecondsInDay))))
  (Transformation|SetActorRotation (Math|Rotator|MakeRotator 0.0 (* (/ _output_get (Variables|TimeConstants|GetSecondsInDay)) 3.6e+02) 0.0)))

(fn ConstructionScript)